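; Game Instance that owns the WeaponManager and handles saving and loading of the player's weapons.
; On Init it constructs the manager and, if a WeaponSave slot exists, initializes it with the saved weapons and the weapon data table.
; Without a save, the manager is created but left uninitialized.
; SaveWeapon writes the manager's current weapons into a fresh BP_Save object in that slot, replacing any previous save.
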(event `self.ReceiveInit`
  (`KismetSystemLibrary.PrintString` "Game Instance Init")
  (bind _returnvalue (`|GenericCreateObject` "/Script/ProjectNull.WeaponManager"))
  (set `self.WeaponManager` _returnvalue)
  (`KismetSystemLibrary.PrintString` "WeaponManager Created")
  (bind _returnvalue_2 (`GameplayStatics.DoesSaveGameExist` "WeaponSave"))
  (if _returnvalue_2
    (`KismetSystemLibrary.PrintString` "セーブデータあります")
    (bind _returnvalue_3 (`GameplayStatics.LoadGameFromSlot` "WeaponSave"))
    (bind _asbp_save (cast `/Game/Title_Tani/SaveGame/BP_Save` _returnvalue_3))
    (`WeaponManager.Initialize` (`self.WeaponManager`) (`/Game/Title_Tani/SaveGame/BP_Save.Weapons` _asbp_save) "/Game/Title_Tani/Data/Weapon/WeaponDataTable.WeaponDataTable")
    (else
      (`KismetSystemLibrary.PrintString` "セーブデータないよー"))))

(fn `SaveWeapon`
  (bind _returnvalue (`GameplayStatics.CreateSaveGameObject` "/Game/Title_Tani/SaveGame/BP_Save.BP_Save_C"))
  (bind _asbp_save (cast `/Game/Title_Tani/SaveGame/BP_Save` _returnvalue))
  (set `/Game/Title_Tani/SaveGame/BP_Save.Weapons` (`WeaponManager.GetWeapons` (`self.WeaponManager`)) _asbp_save)
  (`GameplayStatics.SaveGameToSlot` _asbp_save "WeaponSave")
  (`KismetSystemLibrary.PrintString` "Saved"))